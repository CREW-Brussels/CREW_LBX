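; MoveableItem is an item actor Blueprint that keeps its transform in sync between server and clients.
; The server stores the actor transform on BeginPlay and updates the Transform variable on Tick whenever the actor has moved.
; Clients snap to that RepNotify variable without sweep, both every Tick and in OnRep_Transform, which also prints a debug string.
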(event `self.ReceiveBeginPlay`
  (if (`KismetSystemLibrary.IsServer`)
    (set `self.Transform` (`self.GetTransform`))))

(event `self.ReceiveTick`
  (params (DeltaSeconds :type "Float (single-precision)"))
  (bind _returnvalue (`self.GetTransform`))
  (if (`KismetSystemLibrary.IsServer`)
    (if (not (== _returnvalue (`self.Transform`)))
      (set `self.Transform` _returnvalue))
    (else
      (`self.K2_SetActorTransform` (`self.Transform`)))))

(fn `OnRep_Transform`
  (`KismetSystemLibrary.PrintString` "HelloNotify")
  (if (not (`KismetSystemLibrary.IsServer`))
    (`self.K2_SetActorTransform` (`self.Transform`))))

(fn `UserConstructionScript`)