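; Level manager actor that preloads every entry of the Levels enum as a level instance and switches which ones are shown.
; BeginPlay loads them hidden, mapped by enum, then shows Default.
; Warp, Add and Remove toggle streaming-level visibility and track visible levels in Loaded.
; The "All" events call matching events on every VRTrackingChar, passing a constant ToLevels(0) instead of their Level argument.
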(event `self.ReceiveBeginPlay`
  (bind _default (`self.Default`))
  (bind (_value _returnvalue) (`BlueprintMapLibrary.Map_Find` (`self.Levels`) _default))
  (bind _enumvalue (foreach `/Game/Blueprints/LevelManager/Levels` false)
    (:`LoopBody`
      (bind (_boutsuccess _returnvalue_2) (`LevelStreamingDynamic.LoadLevelInstance` (`|GetEnumeratorNameAsString` _enumvalue) (0.0 0.0 0.0) (struct) "" null))
      (if _boutsuccess
        (set `LevelStreaming.bShouldBeVisible` false _returnvalue_2)
        (`BlueprintMapLibrary.Map_Add` (`self.Levels`) _enumvalue _returnvalue_2)))
    (:`then`
      (if _returnvalue
        (set `LevelStreaming.bShouldBeVisible` true _value)
        (`KismetArrayLibrary.Array_Add` (`self.Loaded`) _default)))))

(event `WarpAll_Event`
  (params (Level :type "/Game/Blueprints/LevelManager/Levels Enum" :default "NewEnumerator0"))
  (bind _outactors (`GameplayStatics.GetAllActorsOfClass` "/CrewVRTracking/Character/VRTrackingChar.VRTrackingChar_C"))
  (for _array_element _outactors
    (`/CrewVRTracking/Character/VRTrackingChar.WarpLevel_Event` _array_element (cast `/CrewVRTracking/Level/Levels` 0))))

(event `AddAll_Event`
  (params (Level :type "/Game/Blueprints/LevelManager/Levels Enum" :default "NewEnumerator0"))
  (bind _outactors (`GameplayStatics.GetAllActorsOfClass` "/CrewVRTracking/Character/VRTrackingChar.VRTrackingChar_C"))
  (for _array_element _outactors
    (`/CrewVRTracking/Character/VRTrackingChar.AddLevel_Event` _array_element (cast `/CrewVRTracking/Level/Levels` 0))))

(event `RemoveAll_Event`
  (params (Level :type "/Game/Blueprints/LevelManager/Levels Enum" :default "NewEnumerator0"))
  (bind _outactors (`GameplayStatics.GetAllActorsOfClass` "/CrewVRTracking/Character/VRTrackingChar.VRTrackingChar_C"))
  (for _array_element _outactors
    (`/CrewVRTracking/Character/VRTrackingChar.RemoveLevel_Event` _array_element (cast `/CrewVRTracking/Level/Levels` 0))))

(fn `Add`
  (params (Level :type "/Game/Blueprints/LevelManager/Levels Enum" :default "NewEnumerator0"))
  (bind (_value _returnvalue) (`BlueprintMapLibrary.Map_Find` (`self.Levels`) Level))
  (`KismetArrayLibrary.Array_Add` (`self.Loaded`) Level)
  (if _returnvalue
    (set `LevelStreaming.bShouldBeVisible` true _value)))

(fn `Remove`
  (params (Level :type "/Game/Blueprints/LevelManager/Levels Enum" :default "NewEnumerator0"))
  (bind _loaded (`self.Loaded`))
  (bind _returnvalue (`KismetArrayLibrary.Array_Find` _loaded Level))
  (bind (_value _returnvalue_2) (`BlueprintMapLibrary.Map_Find` (`self.Levels`) Level))
  (if (>= _returnvalue 0)
    (`|ExecutionSequence`
      (:`then_0`
        (if _returnvalue_2
          (set `LevelStreaming.bShouldBeVisible` false _value)))
      (:`then_1`
        (`KismetArrayLibrary.Array_Remove` _loaded _returnvalue)))))

(fn `UserConstructionScript`)

(fn `Warp`
  (params (Level :type "/Game/Blueprints/LevelManager/Levels Enum" :default "NewEnumerator0"))
  (bind _loaded (`self.Loaded`))
  (bind (_value _returnvalue) (`BlueprintMapLibrary.Map_Find` (`self.Levels`) Level))
  (for _array_element (`self.Loaded`)
    (bind (_value_2 _returnvalue_2) (`BlueprintMapLibrary.Map_Find` (`self.Levels`) _array_element))
    (if _returnvalue_2
      (set `LevelStreaming.bShouldBeVisible` false _value_2)))
  (`KismetArrayLibrary.Array_Clear` _loaded)
  (`KismetArrayLibrary.Array_Add` _loaded Level)
  (if _returnvalue
    (set `LevelStreaming.bShouldBeVisible` true _value)))