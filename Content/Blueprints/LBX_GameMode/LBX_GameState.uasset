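; LBX game state that replicates per-player-group item visibility and applies it to restricted-visibility items.
; The PlayerItemVisibility RepNotify runs its logic only on the server, reading the local player group from LBX_GameInstance.
; It loops over every RestrictedVisibilityItem, setting its root and child visibility by whether that group's entry contains the item's group.
; BeginPlay, Tick and the construction script add no logic.
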(fn `OnRep_PlayerItemVisibility`
  (bind (_playergroup1 _playergroup2 _playergroup3 _playergroup4 _playergroup5 _playergroup6 _playergroup7 _playergroup8) (break `/CrewVRTracking/Items/PlayerItemInteraction` (`self.PlayerItemVisibility`)))
  (if (`KismetSystemLibrary.IsServer`)
    (bind _aslbx_game_instance (cast `/Game/Blueprints/LBX_GameMode/LBX_GameInstance` (`GameplayStatics.GetGameInstance`)))
    (bind _outactors (`GameplayStatics.GetAllActorsOfClass` "/Game/Blueprints/Items/RestrictedVisibilityItem.RestrictedVisibilityItem_C"))
    (for _array_element _outactors
      (`SceneComponent.SetVisibility` (`/Game/Blueprints/Items/Item.DefaultSceneRoot` _array_element) (`KismetArrayLibrary.Array_Contains` (select `/Game/Blueprints/Items/PlayerGroup` (`/Game/Blueprints/LBX_GameMode/LBX_GameInstance.PlayerGroup` _aslbx_game_instance) :`NewEnumerator0` _playergroup1 :`NewEnumerator1` _playergroup2 :`NewEnumerator2` _playergroup3 :`NewEnumerator3` _playergroup4 :`NewEnumerator4` _playergroup5 :`NewEnumerator5` _playergroup6 :`NewEnumerator6` _playergroup7 :`NewEnumerator7` _playergroup8) (`/Game/Blueprints/Items/Item.ItemGroup` _array_element)) true))))

(fn `UserConstructionScript`
  (`parent.UserConstructionScript`))