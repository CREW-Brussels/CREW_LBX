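; BP_SoundTrigger is a sound trigger Blueprint that exposes Play and Stop functions for its Audio component.
; Play fades the sound in when Fade is set, otherwise starts it immediately.
; Stop always fades out when Fade is set; StopOnExit only gates the immediate stop.
; Its own event graph holds only disabled placeholder events, so nothing in this file calls either function.
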(fn `Play`
  (bind _audio (`self.Audio`))
  (if (`self.Fade`)
    (`AudioComponent.FadeIn` _audio (`self.FadeIn`) 1.0 0.0 "Linear")
    (else
      (`AudioComponent.Play` _audio 0.0))))

(fn `Stop`
  (bind _audio (`self.Audio`))
  (if (`self.Fade`)
    (`AudioComponent.FadeOut` _audio (`self.FadeOut`) 0.0 "Linear")
    (elif (`self.StopOnExit`)
      (`AudioComponent.Stop` _audio))))

(fn `UserConstructionScript`
  (`parent.UserConstructionScript`))