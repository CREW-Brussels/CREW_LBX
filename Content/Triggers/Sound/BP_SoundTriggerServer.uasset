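; BP_SoundTriggerServer is a sound trigger that starts and stops its sound only on the server as players enter and leave it.
; On BeginPlay it binds handlers to its inherited Enter and Leave events.
; Each handler checks IsServer before calling Play or Stop, so clients never trigger the sound themselves.
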(event `self.ReceiveBeginPlay`
  (add `/Game/Triggers/BP_Trigger.Enter` (delegate `Enter_Event`))
  (add `/Game/Triggers/BP_Trigger.Leave` (delegate `Leave_Event`)))

(event `Enter_Event`
  (params (Player :type "/Game/Character/VRLBXCharacter Object Reference"))
  (if (`KismetSystemLibrary.IsServer`)
    (`self.Play`)))

(event `Leave_Event`
  (params (Player :type "/Game/Character/VRLBXCharacter Object Reference"))
  (if (`KismetSystemLibrary.IsServer`)
    (`self.Stop`)))

(fn `UserConstructionScript`
  (`parent.UserConstructionScript`))